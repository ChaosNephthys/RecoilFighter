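; BP_ShotManager is a one-shot spawner that fires a scattered burst of BP_Shot actors from the player pawn's location.
; On BeginPlay it plays an explosion emitter at the pawn, then spawns shots in a loop sized by ShotNum.
; Each velocity points from the pawn toward the manager's own location, offset by control-rotation forward plus random spread scaled by ShotDecentralization.
; The manager then destroys itself.
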(event `self.ReceiveBeginPlay`
  (bind _returnvalue (`GameplayStatics.GetPlayerPawn` 0))
  (bind _returnvalue_2 (`self.K2_GetActorLocation` _returnvalue))
  (`/Engine/EditorBlueprintResources/StandardMacros.IsValid` _returnvalue
    (:`Is Valid`
      (`GameplayStatics.SpawnEmitterAtLocation` "/Game/StarterContent/Particles/P_Explosion.P_Explosion" _returnvalue_2)
      (for _ (range (+ (`self.ShotNum`) 1))
        (bind _returnvalue_3 (`|SpawnActorFromClass` "/Game/BP/Shot/BP_Shot.BP_Shot_C" (`KismetMathLibrary.Conv_VectorToTransform` _returnvalue_2) "Undefined" "OverrideRootScale" null null))
        (`/Engine/EditorBlueprintResources/StandardMacros.IsValid` _returnvalue_3
          (:`Is Valid`
            (set `/Game/BP/Shot/BP_Shot.ShotVelocity` (+ (* (`KismetMathLibrary.Normal` (- (`self.K2_GetActorLocation` self) _returnvalue_2)) (`self.ShotVelocitySpeed`)) (* (+ (`KismetMathLibrary.GetForwardVector` (`Pawn.GetControlRotation` (`GameplayStatics.GetPlayerPawn` 0))) (`KismetMathLibrary.RandomUnitVector`)) (`self.ShotDecentralization`))) _returnvalue_3))))
      (`self.K2_DestroyActor`))))

(fn `UserConstructionScript`)