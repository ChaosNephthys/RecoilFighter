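; BP_AttackWarning is a timed attack telegraph that marks an area with a decal, then knocks back characters inside it.
; Tick counts down and feeds the remaining time fraction to the decal's dynamic material.
; At expiry it launches each ThirdPersonCharacter overlapping the sphere outward with an upward-biased, mass-independent velocity impulse, then destroys itself.
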(event `self.ReceiveBeginPlay`
  (bind _returnvalue (`DecalComponent.CreateDynamicMaterialInstance` (`self.Decal`)))
  (set `self.Material` _returnvalue)
  (set `self.TimeLeft` (`self.Time`)))

(event `self.ReceiveTick`
  (params (DeltaSeconds :type "Float (single-precision)"))
  (bind _timeleft (`self.TimeLeft`))
  (bind _output_get (set `self.TimeLeft` (- _timeleft DeltaSeconds)))
  (`MaterialInstanceDynamic.SetScalarParameterValue` (`self.Material`) "TimeLeft" (/ _output_get (`self.Time`)))
  (if (> 0.0 _timeleft)
    (for _array_element (`PrimitiveComponent.GetOverlappingActors` (`self.Sphere`) "/Game/ThirdPersonBP/Blueprints/ThirdPersonCharacter.ThirdPersonCharacter_C")
      (bind _asthird_person_character (cast `/Game/ThirdPersonBP/Blueprints/ThirdPersonCharacter` _array_element))
      (bind (_returnvalue_x _returnvalue_y) (`KismetMathLibrary.BreakVector` (- (`self.K2_GetActorLocation` _asthird_person_character) (`self.K2_GetActorLocation`))))
      (`CharacterMovementComponent.AddImpulse` (`Character.CharacterMovement` _asthird_person_character) (* (`KismetMathLibrary.Normal` (`KismetMathLibrary.MakeVector` _returnvalue_x _returnvalue_y 100.0)) 1000.0) true))
    (`self.K2_DestroyActor`)))

(fn `UserConstructionScript`)