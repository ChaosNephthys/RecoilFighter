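; Boss HP area gimmick that shows a boss's health widget while the player character is inside its box volume.
; On overlap with a ThirdPersonCharacter, it creates an EnemyHp widget bound to the BossEnemy reference and adds it to the viewport, with a flag preventing duplicates.
; Leaving the box removes the widget and resets the flag.
; Tick also removes the widget once the boss is no longer valid.
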(event `self.ReceiveTick`
  (params (DeltaSeconds :type "Float (single-precision)"))
  (bind _widget (`self.widget`))
  (`/Engine/EditorBlueprintResources/StandardMacros.IsValid` (`self.BossEnemy`)
    (:`Is Not Valid`
      (`/Engine/EditorBlueprintResources/StandardMacros.IsValid` _widget
        (:`Is Valid`
          (`Widget.RemoveFromParent` _widget))))))

(event `self.Box.OnComponentBeginOverlap`
  (params (OverlappedComponent :type "PrimitiveComponent Object Reference") (OtherActor :type "Actor Object Reference") (OtherComp :type "PrimitiveComponent Object Reference") (OtherBodyIndex :type Integer) (bFromSweep :type Boolean) (SweepResult :type "HitResult Structure (by ref)"))
  (cast `/Game/ThirdPersonBP/Blueprints/ThirdPersonCharacter` OtherActor)
  (`/Engine/EditorBlueprintResources/StandardMacros.IsValid` (`self.BossEnemy`)
    (:`Is Valid`
      (if (not (`self.AddFlag`))
        (bind _returnvalue (`|CreateWidget` "/Game/BP/Gimmick/EnemyHp.EnemyHp_C"))
        (set `/Game/BP/Gimmick/EnemyHp.Boss` (`self.BossEnemy`) _returnvalue)
        (bind _output_get (set `self.widget` _returnvalue))
        (`UserWidget.AddToViewport` _output_get 0)
        (set `self.AddFlag` true)))))

(event `self.Box.OnComponentEndOverlap`
  (params (OverlappedComponent :type "PrimitiveComponent Object Reference") (OtherActor :type "Actor Object Reference") (OtherComp :type "PrimitiveComponent Object Reference") (OtherBodyIndex :type Integer))
  (bind _widget (`self.widget`))
  (cast `/Game/ThirdPersonBP/Blueprints/ThirdPersonCharacter` OtherActor)
  (`/Engine/EditorBlueprintResources/StandardMacros.IsValid` (`self.BossEnemy`)
    (:`Is Valid`
      (`/Engine/EditorBlueprintResources/StandardMacros.IsValid` _widget
        (:`Is Valid`
          (`Widget.RemoveFromParent` _widget))
        (:`Is Not Valid`
          _))
      (set `self.AddFlag` false))))

(fn `UserConstructionScript`)