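; BP_HealBitStand is a gimmick stand that spawns a heal bit and replaces it after it disappears.
; On BeginPlay it spawns a BP_HealBitStatic at BitPosition, passes it OwnerEnemy, and tints the Cube green through a dynamic M_Shield material.
; While OwnerEnemy is valid and the bit is gone, Tick counts down RespawnTime before spawning a new one.
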(event `self.ReceiveBeginPlay`
  (`parent.ReceiveBeginPlay`)
  (`self.SpawnBit`)
  (bind _returnvalue (`PrimitiveComponent.CreateDynamicMaterialInstance` (`self.Cube`) 0 "/Game/Effects/M_Shield.M_Shield" "None"))
  (`MaterialInstanceDynamic.SetVectorParameterValue` _returnvalue "Emmissive" (make `LinearColor` 0.0 1.0)))

(event `self.ReceiveTick`
  (params (DeltaSeconds :type "Float (single-precision)"))
  (`parent.ReceiveTick` DeltaSeconds)
  (`/Engine/EditorBlueprintResources/StandardMacros.IsValid` (`self.OwnerEnemy`)
    (:`Is Valid`
      (`/Engine/EditorBlueprintResources/StandardMacros.IsValid` (`self.Bit`)
        (:`Is Not Valid`
          (bind _output_get (set `self.Time` (- (`self.Time`) DeltaSeconds)))
          (if (< _output_get 0.0)
            (`self.SpawnBit`)))))))

(event `SpawnBit`
  (bind _returnvalue (`|SpawnActorFromClass` "/Game/BP/Enemy/Bit/BP_HealBitStatic.BP_HealBitStatic_C" (`SceneComponent.K2_GetComponentToWorld` (`self.BitPosition`)) "Undefined" "OverrideRootScale" null null))
  (bind _output_get (set `self.Bit` _returnvalue))
  (set `/Game/BP/Enemy/Bit/BP_BaseBit.OwnerCount` false _output_get)
  (set `/Game/BP/Enemy/Bit/BP_BaseBit.OwnerEnemy` (`self.OwnerEnemy`) _output_get)
  (set `self.Time` (`self.RespawnTime`)))

(fn `UserConstructionScript`
  (`parent.UserConstructionScript`))