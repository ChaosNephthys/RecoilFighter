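; Gimmick gate that spans a wall between two piles and plays a one-time camera-featured reveal when its flag count runs out.
; BeginPlay spawns BP_Wall at the piles' midpoint, rotated and stretched to span them, with a dynamic material.
; Once FlagNum reaches zero, Tick runs a timeline driving the wall's Alpha while the view blends to the gate, then back to the player, and locks the gimmick.
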(event `self.ReceiveBeginPlay`
  (bind _returnvalue_location (`KismetMathLibrary.BreakTransform` (`self.GetTransform` (`self.Pile1`))))
  (bind _returnvalue_location_2 (`KismetMathLibrary.BreakTransform` (`self.GetTransform` (`self.Pile2`))))
  (bind (_returnvalue_roll _returnvalue_pitch _returnvalue_yaw) (`KismetMathLibrary.BreakRotator` (`KismetMathLibrary.FindLookAtRotation` _returnvalue_location _returnvalue_location_2)))
  ;[1 1 1] BeginPlay
  (`parent.ReceiveBeginPlay`)
  (bind _returnvalue (`|SpawnActorFromClass` "/Game/BP/Wall/BP_Wall.BP_Wall_C" (`KismetMathLibrary.MakeTransform` (/ (+ _returnvalue_location _returnvalue_location_2) 2.0) (`KismetMathLibrary.MakeRotator` _returnvalue_roll 0.0 _returnvalue_yaw) (`KismetMathLibrary.MakeVector` (/ (`KismetMathLibrary.Distance2D` (`KismetMathLibrary.Conv_VectorToVector2D` _returnvalue_location) (`KismetMathLibrary.Conv_VectorToVector2D` _returnvalue_location_2)) 100.0) 1.0 1.0)) "Undefined" "OverrideRootScale" null null))
  (bind _output_get (set `self.Wall` _returnvalue))
  (bind _returnvalue_2 (`PrimitiveComponent.CreateDynamicMaterialInstance` (`/Game/BP/Wall/BP_Wall.Cube` _output_get) 0 "/Game/BP/Wall/M_Wall.M_Wall" "None"))
  (bind _output_get_2 (set `self.Material` _returnvalue_2))
  (`MaterialInstanceDynamic.SetVectorParameterValue` _output_get_2 "Color" (make `LinearColor` 1.0 1.0 0.0 1.0)))

(event `self.ReceiveTick`
  (params (DeltaSeconds :type "Float (single-precision)"))
  (bind _flagnum (`self.FlagNum`))
  (`parent.ReceiveTick` DeltaSeconds)
  (`KismetSystemLibrary.PrintString` (`KismetStringLibrary.Conv_DoubleToString` _flagnum) true true (struct :`G` 0.66 :`B` 1.0 :`A` 1.0) 0.0)
  (if (and (>= 0.0 _flagnum) (not (`self.GimmickLock`)))
    (bind (_direction _general) (`Timeline|タイムライン_0`)
      (:`Update`
        (`|ExecutionSequence`
          (:`then_0`
            (`/Engine/EditorBlueprintResources/StandardMacros.DoOnce` false
              (:`Completed`
                (`PlayerController.SetViewTargetWithBlend` (`GameplayStatics.GetPlayerController` 0) self (`self.CameraSpeed`) "VTBlend_Linear" 0.0 false))))
          (:`then_1`
            (`MaterialInstanceDynamic.SetScalarParameterValue` (`self.Material`) "Alpha" _general))))
      (:`Finished`
        (`PlayerController.SetViewTargetWithBlend` (`GameplayStatics.GetPlayerController` 0) (cast `/Game/ThirdPersonBP/Blueprints/ThirdPersonCharacter` (`GameplayStatics.GetPlayerPawn` 0) :!pure true) (`self.CameraSpeed`) "VTBlend_Linear" 0.0 false)
        (set `self.GimmickLock` true)))))

(fn `UserConstructionScript`
  (`parent.UserConstructionScript`))