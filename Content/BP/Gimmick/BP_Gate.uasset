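; BP_Gate is a two-panel gate gimmick that opens while the view blends to the gate itself.
; On Tick, a set IsLanch flag disables both panels' collision and plays the GateOpen timeline, which slides them apart along Y while narrowing them.
; A DoOnce blends the view to the gate on the first update; on finish it blends to the ThirdPersonCharacter's Camera, both using CameraSpeed.
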(event `self.ReceiveTick`
  (params (DeltaSeconds :type "Float (single-precision)"))
  (bind _gate1 (`self.Gate1`))
  (bind _gate2 (`self.Gate2`))
  (`parent.ReceiveTick` DeltaSeconds)
  (if (`self.IsLanch`)
    (`PrimitiveComponent.SetCollisionEnabled` (`self.Gate1`) "NoCollision")
    (`PrimitiveComponent.SetCollisionEnabled` (`self.Gate2`) "NoCollision")
    (bind (_direction _general) (`Timeline|GateOpen`)
      (:`Update`
        (`|ExecutionSequence`
          (:`then_0`
            (`SceneComponent.K2_SetRelativeLocation` _gate1 (`KismetMathLibrary.MakeVector` 0.0 (+ (* _general 150.0) 100.0) 150.0) false false)
            (bind _returnvalue (- 2.0 _general))
            (`SceneComponent.SetRelativeScale3D` _gate1 (`KismetMathLibrary.MakeVector` 0.5 _returnvalue 3.0))
            (`/Engine/EditorBlueprintResources/StandardMacros.DoOnce` false
              (:`Completed`
                (`PlayerController.SetViewTargetWithBlend` (`GameplayStatics.GetPlayerController` 0) self (`self.CameraSpeed`) "VTBlend_Linear" 0.0 false))))
          (:`then_1`
            (`SceneComponent.K2_SetRelativeLocation` _gate2 (`KismetMathLibrary.MakeVector` 0.0 (+ (* _general -150.0) -100.0) 150.0) false false)
            (`SceneComponent.SetRelativeScale3D` _gate2 (`KismetMathLibrary.MakeVector` 0.5 _returnvalue 3.0)))))
      (:`Finished`
        (`PlayerController.SetViewTargetWithBlend` (`GameplayStatics.GetPlayerController` 0) (`/Game/ThirdPersonBP/Blueprints/ThirdPersonCharacter.Camera` (cast `/Game/ThirdPersonBP/Blueprints/ThirdPersonCharacter` (`GameplayStatics.GetPlayerPawn` 0) :!pure true)) (`self.CameraSpeed`) "VTBlend_Linear" 0.0 false)))))

(fn `UserConstructionScript`
  (`parent.UserConstructionScript`))