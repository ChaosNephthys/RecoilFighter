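; Moving floor gimmick that oscillates a Cube between the actor's root and a Scene component marking the far end.
; BeginPlay places the Cube and sets the Niagara "Beam End" to the far end's location.
; Tick advances Time by Speed and drives an unswept lerp with a remapped sine while FlagNum is zero or below.
; A positive FlagNum freezes the Cube and pins Time at -1, so movement resumes from that phase.
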(event `self.ReceiveBeginPlay`
  (`parent.ReceiveBeginPlay`)
  (`NiagaraComponent.SetNiagaraVariableVec3` (`self.Niagara`) "Beam End" (`SceneComponent.K2_GetComponentLocation` (`self.Scene`)))
  (`SceneComponent.K2_SetWorldLocation` (`self.Cube`) (`KismetMathLibrary.VLerp` (`SceneComponent.K2_GetComponentLocation` (`self.DefaultSceneRoot`)) (`SceneComponent.K2_GetComponentLocation` (`self.Scene`)) (+ (/ (`KismetMathLibrary.Sin` (`self.time`)) 2.0) 0.5)) false false))

(event `self.ReceiveTick`
  (params (DeltaSeconds :type "Float (single-precision)"))
  (`parent.ReceiveTick` DeltaSeconds)
  (if (<= (`self.FlagNum`) 0.0)
    (bind _output_get (set `self.time` (+ (* DeltaSeconds (`self.speed`)) (`self.time`))))
    (`SceneComponent.K2_SetWorldLocation` (`self.Cube`) (`KismetMathLibrary.VLerp` (`SceneComponent.K2_GetComponentLocation` (`self.DefaultSceneRoot`)) (`SceneComponent.K2_GetComponentLocation` (`self.Scene`)) (+ (/ (`KismetMathLibrary.Sin` _output_get) 2.0) 0.5)) false false)
    (else
      (set `self.time` -1.0))))

(fn `UserConstructionScript`
  (`parent.UserConstructionScript`))