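; Combat arena gimmick that walls players in until its enemy counter, FlagNum, reaches zero, then fades and destroys itself.
; On BeginPlay it spawns box-scaled BP_Wall sides with optional floor and ceiling, counts overlapping BaseEnemy actors and registers itself with them.
; Tick fades wall materials with player presence, toggling collision at full or zero alpha.
; Registered enemies leaving the volume are teleported toward the centre after a delay, using a randomized line trace.
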(event `self.ReceiveBeginPlay`
  (bind _cube (`self.Cube`))
  (bind _cube1 (`self.Cube1`))
  (bind _cube2 (`self.Cube2`))
  (bind _cube3 (`self.Cube3`))
  (bind _overlappingactors (`PrimitiveComponent.GetOverlappingActors` (`self.Virtual`) "/Game/BP/Enemy/BaseEnemy.BaseEnemy_C"))
  (bind (_returnvalue_x _returnvalue_y _returnvalue_z) (`KismetMathLibrary.BreakVector` (`SceneComponent.K2_GetComponentScale` _cube3)))
  (bind (_returnvalue_x_2 _returnvalue_y_2 _returnvalue_z_2) (`KismetMathLibrary.BreakVector` (`SceneComponent.K2_GetComponentScale` _cube)))
  (bind (_returnvalue_x_3 _returnvalue_y_3 _returnvalue_z_3) (`KismetMathLibrary.BreakVector` (`SceneComponent.K2_GetComponentScale` _cube1)))
  (bind (_returnvalue_x_4 _returnvalue_y_4 _returnvalue_z_4) (`KismetMathLibrary.BreakVector` (`SceneComponent.K2_GetComponentScale` _cube2)))
  (`parent.ReceiveBeginPlay`)
  (`self.MakeWall`)
  (`self.WallHitOff`)
  (`KismetSystemLibrary.Delay` 0.1)
  (for _array_element _overlappingactors
    (bind _asbase_enemy (cast `/Game/BP/Enemy/BaseEnemy` _array_element))
    (`KismetArrayLibrary.Array_Add` (`/Game/BP/Enemy/BaseEnemy.LanchGimmick` _asbase_enemy) self))
  (set `self.FlagNum` (`KismetMathLibrary.Conv_IntToDouble` (`KismetArrayLibrary.Array_Length` _overlappingactors)))
  (`SceneComponent.SetWorldScale3D` _cube (`KismetMathLibrary.MakeVector` (`self.EnemyWallScale`) _returnvalue_y_2 _returnvalue_z_2))
  (`SceneComponent.SetWorldScale3D` _cube1 (`KismetMathLibrary.MakeVector` (`self.EnemyWallScale`) _returnvalue_y_3 _returnvalue_z_3))
  (`SceneComponent.SetWorldScale3D` _cube2 (`KismetMathLibrary.MakeVector` _returnvalue_x_4 (`self.EnemyWallScale`) _returnvalue_z_4))
  (`SceneComponent.SetWorldScale3D` _cube3 (`KismetMathLibrary.MakeVector` _returnvalue_x (`self.EnemyWallScale`) _returnvalue_z)))

(event `self.ReceiveTick`
  (params (DeltaSeconds :type "Float (single-precision)"))
  (bind _alpha (`self.Alpha`))
  (bind _returnvalue (* DeltaSeconds (`self.WallSpeed`)))
  (`parent.ReceiveTick` DeltaSeconds)
  (if (`self.Lock`)
    _
    (elif (>= 0.0 (`self.FlagNum`))
      ;[1 1 1] 壁の消滅
      (bind (_direction _alpha_2) (`Timeline|Time`)
        (:`Update`
          (for _array_element (`self.Material`)
            (`MaterialInstanceDynamic.SetScalarParameterValue` _array_element "Alpha" (* _alpha_2 0.2))))
        (:`Finished`
          (set `self.Lock` true)
          (for _array_element_2 (`self.Wall`)
            (`self.K2_DestroyActor` _array_element_2))
          (`self.K2_DestroyActor`)))
      (else
        ;[1 1 1] 壁のON/OFF切り替え
        (for _array_element_3 (`self.Material`)
          (`MaterialInstanceDynamic.SetScalarParameterValue` _array_element_3 "Alpha" (* (`self.Alpha`) 0.2)))
        (if (> (`KismetArrayLibrary.Array_Length` (`self.Player`)) 0)
          (set `self.Alpha` (+ _returnvalue _alpha))
          (else
            (set `self.Alpha` (- _alpha _returnvalue))))
        (bind _output_get (set `self.Alpha` (`KismetMathLibrary.FClamp` (`self.Alpha`))))
        (if (== _output_get 0.0)
          (`self.WallHitOff`)
          (elif (== _output_get 1.0)
            (`self.WallHitOn`)))))))

(event `self.Virtual.OnComponentBeginOverlap`
  (params (OverlappedComponent :type "PrimitiveComponent Object Reference") (OtherActor :type "Actor Object Reference") (OtherComp :type "PrimitiveComponent Object Reference") (OtherBodyIndex :type Integer) (bFromSweep :type Boolean) (SweepResult :type "HitResult Structure (by ref)"))
  (if (not (`self.Lock`))
    (bind _asthird_person_character (cast `/Game/ThirdPersonBP/Blueprints/ThirdPersonCharacter` OtherActor))
    (if (== (`Character.CapsuleComponent` _asthird_person_character) OtherComp)
      (`KismetArrayLibrary.Array_AddUnique` (`self.Player`) _asthird_person_character))))

(event `self.Virtual.OnComponentEndOverlap`
  (params (OverlappedComponent :type "PrimitiveComponent Object Reference") (OtherActor :type "Actor Object Reference") (OtherComp :type "PrimitiveComponent Object Reference") (OtherBodyIndex :type Integer))
  (bind _returnvalue (`self.K2_GetActorLocation`))
  (bind _returnvalue_2 (* (`KismetMathLibrary.Sin` (`KismetMathLibrary.MultiplyByPi` (`KismetMathLibrary.RandomFloat`))) 100.0))
  (bind _returnvalue_3 (* (`KismetMathLibrary.Cos` (`KismetMathLibrary.MultiplyByPi` (`KismetMathLibrary.RandomFloat`))) 100.0))
  (if (not (`self.Lock`))
    (bind _asthird_person_character (cast `/Game/ThirdPersonBP/Blueprints/ThirdPersonCharacter` OtherActor)
      (:`then`
        (if (== (`Character.CapsuleComponent` _asthird_person_character) OtherComp)
          (`KismetArrayLibrary.Array_RemoveItem` (`self.Player`) _asthird_person_character)))
      (:`CastFailed`
        (bind _asbase_enemy (cast `/Game/BP/Enemy/BaseEnemy` OtherActor))
        (if (`KismetArrayLibrary.Array_Contains` (`/Game/BP/Enemy/BaseEnemy.LanchGimmick` _asbase_enemy) self)
          (`KismetSystemLibrary.Delay` 0.5)
          (`/Engine/EditorBlueprintResources/StandardMacros.IsValid` _asbase_enemy
            (:`Is Valid`
              (bind _outhit (`KismetSystemLibrary.LineTraceSingle` (+ _returnvalue (`KismetMathLibrary.MakeVector` _returnvalue_2 _returnvalue_3)) (+ _returnvalue (`KismetMathLibrary.MakeVector` _returnvalue_2 _returnvalue_3 100.0)) "TraceTypeQuery3"))
              (`SceneComponent.K2_SetWorldLocation` (`Character.CapsuleComponent` _asbase_enemy) (`.Location` (`GameplayStatics.BreakHitResult` _outhit)) false true))))))))

(event `AddWallList`
  (params (Wall :type "/Game/BP/Wall/BP_Wall Object Reference"))
  (`KismetArrayLibrary.Array_Add` (`self.Wall`) Wall)
  (bind _returnvalue (`PrimitiveComponent.CreateDynamicMaterialInstance` (`/Game/BP/Wall/BP_Wall.Cube` Wall) 0 "/Game/BP/Wall/M_Wall.M_Wall" "None"))
  (`KismetArrayLibrary.Array_Add` (`self.Material`) _returnvalue))

(event `MakeWall`
  (bind _defaultsceneroot (`self.DefaultSceneRoot`))
  (bind _returnvalue (`SceneComponent.K2_GetComponentToWorld` _defaultsceneroot))
  (bind _returnvalue_2 (`SceneComponent.K2_GetComponentLocation` _defaultsceneroot))
  (bind _returnvalue_3 (`KismetMathLibrary.MakeVector` (.x (.scale _returnvalue)) (.y (.scale _returnvalue)) 0.01))
  (bind _returnvalue_4 (`KismetMathLibrary.MakeVector` 0.01 (.y (.scale _returnvalue)) (.z (.scale _returnvalue))))
  (bind _returnvalue_5 (`KismetMathLibrary.MakeVector` (.x (.scale _returnvalue)) 0.01 (.z (.scale _returnvalue))))
  (bind _returnvalue_6 (* (`KismetMathLibrary.MakeVector` 0.0 0.0 (.z (.scale _returnvalue))) 50))
  (bind _returnvalue_7 (* (`KismetMathLibrary.MakeVector` (.x (.scale _returnvalue))) 50))
  (bind _returnvalue_8 (* (`KismetMathLibrary.MakeVector` 0.0 (.y (.scale _returnvalue))) 50))
  ;[1 1 1] 壁の初期生成
  (`|ExecutionSequence`
    (:`then_0`
      (bind _returnvalue_9 (`|SpawnActorFromClass` "/Game/BP/Wall/BP_Wall.BP_Wall_C" (`KismetMathLibrary.MakeTransform` (+ _returnvalue_2 _returnvalue_7) (struct) _returnvalue_4) "Undefined" "OverrideRootScale" null null))
      (`self.AddWallList` _returnvalue_9))
    (:`then_1`
      (bind _returnvalue_10 (`|SpawnActorFromClass` "/Game/BP/Wall/BP_Wall.BP_Wall_C" (`KismetMathLibrary.MakeTransform` (- _returnvalue_2 _returnvalue_7) (struct) _returnvalue_4) "Undefined" "OverrideRootScale" null null))
      (`self.AddWallList` _returnvalue_10))
    (:`then_2`
      (bind _returnvalue_11 (`|SpawnActorFromClass` "/Game/BP/Wall/BP_Wall.BP_Wall_C" (`KismetMathLibrary.MakeTransform` (+ _returnvalue_2 _returnvalue_8) (struct) _returnvalue_5) "Undefined" "OverrideRootScale" null null))
      (`self.AddWallList` _returnvalue_11))
    (:`then_3`
      (bind _returnvalue_12 (`|SpawnActorFromClass` "/Game/BP/Wall/BP_Wall.BP_Wall_C" (`KismetMathLibrary.MakeTransform` (- _returnvalue_2 _returnvalue_8) (struct) _returnvalue_5) "Undefined" "OverrideRootScale" null null))
      (`self.AddWallList` _returnvalue_12))
    (:`then_4`
      (if (not (`self.DisableCeiling`))
        (bind _returnvalue_13 (`|SpawnActorFromClass` "/Game/BP/Wall/BP_Wall.BP_Wall_C" (`KismetMathLibrary.MakeTransform` (+ _returnvalue_2 _returnvalue_6) (struct) _returnvalue_3) "Undefined" "OverrideRootScale" null null))
        (`self.AddWallList` _returnvalue_13)))
    (:`then_5`
      (if (not (`self.DisableFloor`))
        (bind _returnvalue_14 (`|SpawnActorFromClass` "/Game/BP/Wall/BP_Wall.BP_Wall_C" (`KismetMathLibrary.MakeTransform` (- _returnvalue_2 _returnvalue_6) (struct) _returnvalue_3) "Undefined" "OverrideRootScale" null null))
        (`self.AddWallList` _returnvalue_14)))))

(event `WallHitOn`
  (for _array_element (`self.Wall`)
    (`PrimitiveComponent.SetCollisionEnabled` (`/Game/BP/Wall/BP_Wall.Cube` _array_element) "QueryOnly")))

(event `WallHitOff`
  (for _array_element (`self.Wall`)
    (`PrimitiveComponent.SetCollisionEnabled` (`/Game/BP/Wall/BP_Wall.Cube` _array_element) "NoCollision")))

(fn `UserConstructionScript`
  (`parent.UserConstructionScript`))