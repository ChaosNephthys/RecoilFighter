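; BP_TutorialBalloon is a shootable balloon gimmick, named for the tutorial, that can be chained to other gimmicks.
; Tick keeps its Sphere hidden and without collision while FlagNum is above zero, and shows it with collision otherwise.
; When a BP_Shot overlaps the Sphere, it decrements FlagNum on each ChainGimmick entry and destroys itself, so FlagNum acts as a countdown gate.
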(event `self.ReceiveTick`
  (params (DeltaSeconds :type "Float (single-precision)"))
  (bind _sphere (`self.Sphere`))
  (`parent.ReceiveTick` DeltaSeconds)
  (if (> (`self.FlagNum`) 0.0)
    (`SceneComponent.SetHiddenInGame` _sphere true false)
    (`PrimitiveComponent.SetCollisionEnabled` _sphere "NoCollision")
    (else
      (`SceneComponent.SetHiddenInGame` _sphere false false)
      (`PrimitiveComponent.SetCollisionEnabled` _sphere "QueryAndPhysics"))))

(event `self.Sphere.OnComponentBeginOverlap`
  (params (OverlappedComponent :type "PrimitiveComponent Object Reference") (OtherActor :type "Actor Object Reference") (OtherComp :type "PrimitiveComponent Object Reference") (OtherBodyIndex :type Integer) (bFromSweep :type Boolean) (SweepResult :type "HitResult Structure (by ref)"))
  (cast `/Game/BP/Shot/BP_Shot` OtherActor)
  (for _array_element (`self.ChainGimmick`)
    (set `/Game/BP/Gimmick/BP_BaseGimmick.FlagNum` (- (`/Game/BP/Gimmick/BP_BaseGimmick.FlagNum` _array_element) 1.0) _array_element))
  (`self.K2_DestroyActor`))

(fn `UserConstructionScript`
  (`parent.UserConstructionScript`))