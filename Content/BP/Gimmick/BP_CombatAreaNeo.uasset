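; BP_CombatAreaNeo is a combat arena gimmick that encloses an area with ghost walls until its flag count reaches zero.
; On BeginPlay it spawns inward-facing BP_GhostWall actors from placeholder components, with optional floor and ceiling.
; It then registers itself with overlapping BaseEnemy actors' LanchGimmick and sets FlagNum to their count.
; Tick watches FlagNum, which is not decremented here, then runs a timeline to shrink and destroy the walls.
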(event `self.ReceiveBeginPlay`
  (bind _overlappingactors (`PrimitiveComponent.GetOverlappingActors` (`self.Virtual`) "/Game/BP/Enemy/BaseEnemy.BaseEnemy_C"))
  (`parent.ReceiveBeginPlay`)
  (`self.MakeWall`)
  (`KismetSystemLibrary.Delay` 0.1)
  (for _array_element _overlappingactors
    (bind _asbase_enemy (cast `/Game/BP/Enemy/BaseEnemy` _array_element))
    (`KismetArrayLibrary.Array_Add` (`/Game/BP/Enemy/BaseEnemy.LanchGimmick` _asbase_enemy) self))
  (set `self.FlagNum` (`KismetMathLibrary.Conv_IntToDouble` (`KismetArrayLibrary.Array_Length` _overlappingactors))))

(event `self.ReceiveTick`
  (params (DeltaSeconds :type "Float (single-precision)"))
  (`parent.ReceiveTick` DeltaSeconds)
  (if (`self.Lock`)
    _
    (elif (>= 0.0 (`self.FlagNum`))
      (for _array_element (`self.Wall`)
        (set `/Game/BP/Wall/BP_GhostWall.AnimLock` true _array_element)
        ;[1 1 1] 壁の消滅
        (bind (_direction _alpha) (`Timeline|Time`)
          (:`Update`
            (for _array_element_2 (`self.Wall`)
              (`/Game/BP/Wall/BP_GhostWall.SetDeleteScale` _array_element_2 _alpha)))
          (:`Finished`
            (set `self.Lock` true)
            (for _array_element_3 (`self.Wall`)
              (`self.K2_DestroyActor` _array_element_3))))))))

(event `MakeWall`
  (`self.MakeGhostWall` (`self.Cube`))
  (`self.MakeGhostWall` (`self.Cube1`))
  (`self.MakeGhostWall` (`self.Cube2`))
  (`self.MakeGhostWall` (`self.Cube3`))
  (if (not (`self.DisableFloor`))
    (`self.MakeGhostWall` (`self.Froor`)))
  (if (not (`self.DisableCeiling`))
    (`self.MakeGhostWall` (`self.Ceiling`))))

(event `MakeGhostWall`
  (params (NewParam :type "StaticMeshComponent Object Reference"))
  (bind _returnvalue (`SceneComponent.K2_GetComponentToWorld` NewParam))
  (bind _returnvalue_2 (`|SpawnActorFromClass` "/Game/BP/Wall/BP_GhostWall.BP_GhostWall_C" _returnvalue "Undefined" "OverrideRootScale" null null))
  (`KismetArrayLibrary.Array_Add` (`self.Wall`) _returnvalue_2)
  (set `/Game/BP/Wall/BP_GhostWall.NormalVector` (`KismetMathLibrary.Normal` (- (`self.K2_GetActorLocation`) (.location _returnvalue))) _returnvalue_2))

(fn `UserConstructionScript`
  (`parent.UserConstructionScript`))