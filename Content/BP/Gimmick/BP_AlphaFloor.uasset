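; BP_AlphaFloor is a gimmick floor that fades its cube mesh through a material Alpha parameter, driven by FlagNum.
; BeginPlay creates a dynamic instance of M_Floor_Alpha on the cube.
; Each Tick lowers Alpha while FlagNum is positive and raises it otherwise, clamped between zero and one, then writes it to the material.
; FlagNum is only read here, and collision is never changed.
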(event `self.ReceiveBeginPlay`
  (`parent.ReceiveBeginPlay`)
  (bind _returnvalue (`PrimitiveComponent.CreateDynamicMaterialInstance` (`self.Cube`) 0 "/Game/BP/Wall/M_Floor_Alpha.M_Floor_Alpha" "None"))
  (set `self.Material` _returnvalue))

(event `self.ReceiveActorBeginOverlap`
  (params (OtherActor :type "Actor Object Reference"))
  (`parent.ReceiveActorBeginOverlap` OtherActor))

(event `self.ReceiveTick`
  (params (DeltaSeconds :type "Float (single-precision)"))
  (bind _alpha (`self.Alpha`))
  (`parent.ReceiveTick` DeltaSeconds)
  (if (> (`self.FlagNum`) 0.0)
    (set `self.Alpha` (- _alpha DeltaSeconds))
    (else
      (set `self.Alpha` (+ _alpha DeltaSeconds))))
  (bind _output_get (set `self.Alpha` (`KismetMathLibrary.FClamp` (`self.Alpha`))))
  (`MaterialInstanceDynamic.SetScalarParameterValue` (`self.Material`) "Alpha" _output_get))

(fn `UserConstructionScript`
  (`parent.UserConstructionScript`))