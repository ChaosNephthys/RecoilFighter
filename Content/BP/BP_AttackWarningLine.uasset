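; BP_AttackWarningLine is a short-lived decal actor that, judging by its name, marks the line of an incoming attack.
; On BeginPlay it creates a dynamic material instance from its decal.
; Tick accumulates time to drive the material's Length parameter from zero to full over the first second, then destroys the actor once two seconds have passed.
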(event `self.ReceiveBeginPlay`
  (bind _returnvalue (`DecalComponent.CreateDynamicMaterialInstance` (`self.Decal`)))
  (set `self.Material` _returnvalue))

(event `self.ReceiveTick`
  (params (DeltaSeconds :type "Float (single-precision)"))
  (bind _time (`self.Time`))
  (set `self.Time` (+ DeltaSeconds _time))
  (`MaterialInstanceDynamic.SetScalarParameterValue` (`self.Material`) "Length" (`KismetMathLibrary.FClamp` _time))
  (if (> _time 2.0)
    (`self.K2_DestroyActor`)))

(fn `UserConstructionScript`)