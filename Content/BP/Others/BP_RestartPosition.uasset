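; BP_RestartPosition is a checkpoint actor that sets the player's restart position and heals them on contact.
; The first capsule overlap by a ThirdPersonCharacter, gated by DoOnce, stores the actor's location as that character's RestartPosition and applies a very large heal.
; It then plays a ColorShift timeline that drives the Shift parameter on the plane's dynamic M_Frag material.
; The enlarged plane spins continuously on Tick.
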(event `self.ReceiveBeginPlay`
  (`SceneComponent.SetWorldScale3D` (`self.Plane`) (4.0 4.0 4.0))
  (bind _returnvalue (`PrimitiveComponent.CreateDynamicMaterialInstance` (`self.Plane`) 0 "/Game/BP/Wall/M_Frag.M_Frag" "None"))
  (set `self.Material` _returnvalue))

(event `self.ReceiveActorBeginOverlap`
  (params (OtherActor :type "Actor Object Reference")))

(event `self.ReceiveTick`
  (params (DeltaSeconds :type "Float (single-precision)"))
  (`SceneComponent.K2_AddLocalRotation` (`self.Plane`) (* (`KismetMathLibrary.MakeRotator` 0.0 45.0) DeltaSeconds) false false))

(event `self.Capsule.OnComponentBeginOverlap`
  (params (OverlappedComponent :type "PrimitiveComponent Object Reference") (OtherActor :type "Actor Object Reference") (OtherComp :type "PrimitiveComponent Object Reference") (OtherBodyIndex :type Integer) (bFromSweep :type Boolean) (SweepResult :type "HitResult Structure (by ref)"))
  (bind _asthird_person_character (cast `/Game/ThirdPersonBP/Blueprints/ThirdPersonCharacter` OtherActor))
  (`/Engine/EditorBlueprintResources/StandardMacros.DoOnce` false
    (:`Completed`
      (set `/Game/ThirdPersonBP/Blueprints/ThirdPersonCharacter.RestartPosition` (`self.K2_GetActorLocation`) _asthird_person_character)
      (`/Game/ThirdPersonBP/Blueprints/ThirdPersonCharacter.Heal` _asthird_person_character 9999)
      (bind (_direction _color) (`Timeline|ColorShift`)
        (:`Update`
          (`MaterialInstanceDynamic.SetScalarParameterValue` (`self.Material`) "Shift" _color))))))

(fn `UserConstructionScript`)