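; BP_WallPolygon is an actor that builds a closed regular-polygon wall from BP_WallPile actors at BeginPlay.
; With at least three vertices, it spawns piles at equal yaw steps, Distance from the world origin, taking Z scale from its root.
; Each pile stores its predecessor in ConnectPile, and the first links to the last to close the ring.
; CreateWall then runs on every pile once all links exist.
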(event `self.ReceiveBeginPlay`
  (bind _numberofvertices (`self.NumberOfVertices`))
  (bind _back (`self.Back`))
  (bind (_returnvalue_x _returnvalue_y _returnvalue_z) (`KismetMathLibrary.BreakVector` (`SceneComponent.K2_GetComponentScale` (`self.DefaultSceneRoot`))))
  (if (>= _numberofvertices 3)
    (for _index (range _numberofvertices)
      (bind _returnvalue (`|SpawnActorFromClass` "/Game/BP/Wall/BP_WallPile.BP_WallPile_C" (`KismetMathLibrary.MakeTransform` (* (`KismetMathLibrary.GreaterGreater_VectorRotator` (`KismetMathLibrary.Vector_Forward`) (`KismetMathLibrary.MakeRotator` 0.0 0.0 (* _index (/ 360.0 (`KismetMathLibrary.Conv_IntToDouble` (`self.NumberOfVertices`)))))) (`self.Distance`)) (struct) (`KismetMathLibrary.MakeVector` 0.0 0.0 _returnvalue_z)) "Undefined" "OverrideRootScale" null null))
      (`|ExecutionSequence`
        (:`then_0`
          (`/Engine/EditorBlueprintResources/StandardMacros.IsValid` _back
            (:`Is Valid`
              (`KismetArrayLibrary.Array_Add` (`/Game/BP/Wall/BP_WallPile.ConnectPile` _returnvalue) _back))
            (:`Is Not Valid`
              _))
          (set `self.Back` _returnvalue))
        (:`then_1`
          (`KismetArrayLibrary.Array_Add` (`self.Pile`) _returnvalue))
        (:`then_2`
          (if (== _index 0)
            (set `self.Front` _returnvalue)))))
    (`KismetArrayLibrary.Array_Add` (`/Game/BP/Wall/BP_WallPile.ConnectPile` (`self.Front`)) (`self.Back`))
    (for _array_element (`self.Pile`)
      (`/Game/BP/Wall/BP_WallPile.CreateWall` _array_element))))

(fn `UserConstructionScript`)