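; BP_WallPile is a wall post actor that spawns connecting BP_Wall segments to linked piles when play begins.
; CreateWall loops over the valid entries in ConnectPile and spawns a wall at the midpoint between this pile and each target.
; Each wall takes its yaw from a look-at rotation, stretches in X by 2D distance assuming a 100-unit base length, and copies the root's Z scale.
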(event `self.ReceiveBeginPlay`
  (`self.CreateWall`))

(event `CreateWall`
  (bind _returnvalue_location (`KismetMathLibrary.BreakTransform` (`self.GetTransform`)))
  (bind _connectpile (`self.ConnectPile`))
  (bind (_returnvalue_x _returnvalue_y _returnvalue_z) (`KismetMathLibrary.BreakVector` (`SceneComponent.K2_GetComponentScale` (`self.DefaultSceneRoot`))))
  (if (> (`KismetArrayLibrary.Array_Length` _connectpile) 0)
    (for _array_element _connectpile
      (`/Engine/EditorBlueprintResources/StandardMacros.IsValid` _array_element
        (:`Is Valid`
          (bind _returnvalue_location_2 (`KismetMathLibrary.BreakTransform` (`self.GetTransform` _array_element)))
          (bind (_returnvalue_roll _returnvalue_pitch _returnvalue_yaw) (`KismetMathLibrary.BreakRotator` (`KismetMathLibrary.FindLookAtRotation` _returnvalue_location _returnvalue_location_2)))
          (`|SpawnActorFromClass` "/Game/BP/Wall/BP_Wall.BP_Wall_C" (`KismetMathLibrary.MakeTransform` (/ (+ _returnvalue_location _returnvalue_location_2) 2.0) (`KismetMathLibrary.MakeRotator` _returnvalue_roll 0.0 _returnvalue_yaw) (`KismetMathLibrary.MakeVector` (/ (`KismetMathLibrary.Distance2D` (`KismetMathLibrary.Conv_VectorToVector2D` _returnvalue_location) (`KismetMathLibrary.Conv_VectorToVector2D` _returnvalue_location_2)) 100.0) 1.0 _returnvalue_z)) "Undefined" "OverrideRootScale" null null))))))

(fn `UserConstructionScript`)