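; BP_GhostWall is a one-way wall that blocks from its normal side and lets players through from behind.
; Tick fades the dynamic material's Alpha over a second by which side player pawn 0 is on.
; Separately, the server disables cube collision whenever any player is behind and within range of the infinite plane, so that opening is not per-player.
; SetDeleteScale lerps cube scale between zero and its stored default.
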(event `self.ReceiveBeginPlay`
  (bind (_returnvalue_location _returnvalue_rotation _returnvalue_scale) (`KismetMathLibrary.BreakTransform` (`self.GetTransform`)))
  (bind _returnvalue (`PrimitiveComponent.CreateDynamicMaterialInstance` (`self.Cube`) 0 "/Game/BP/Wall/M_Wall.M_Wall" "None"))
  (`KismetArrayLibrary.Array_Add` (`self.Material`) _returnvalue)
  (if (`self.ForwardNormal`)
    (set `self.NormalVector` (`self.GetActorForwardVector`))
    (set `self.DefaltScale` _returnvalue_scale)))

(event `self.ReceiveTick`
  (params (DeltaSeconds :type "Float (single-precision)"))
  (bind _blocktime (`self.BlockTime`))
  (`|ExecutionSequence`
    (:`then_0`
      (if (not (`self.AnimLock`))
        (for _array_element (`self.Material`)
          (`MaterialInstanceDynamic.SetScalarParameterValue` _array_element "Alpha" (+ (* (`self.BlockTime`) 0.95) 0.05)))))
    (:`then_1`
      ;[1 1 1] ローカル上の見た目変更
      (if (> (`KismetMathLibrary.Dot_VectorVector` (`self.NormalVector`) (- (`self.K2_GetActorLocation` (`GameplayStatics.GetPlayerPawn` 0)) (`self.K2_GetActorLocation`))) 0.0)
        (set `self.BlockTime` (`KismetMathLibrary.FClamp` (+ _blocktime DeltaSeconds)))
        (else
          (set `self.BlockTime` (`KismetMathLibrary.FClamp` (- _blocktime DeltaSeconds))))))
    (:`then_2`
      ;[1 1 1] サーバー側の当たり判定変更
      (if (`KismetSystemLibrary.IsServer`)
        (bind _returnvalue (`GameModeBase.GetNumPlayers` (`GameplayStatics.GetGameMode`)))
        (`PrimitiveComponent.SetCollisionEnabled` (`self.Cube`) "QueryAndPhysics")
        (for _index (range _returnvalue)
          (bind _returnvalue_2 (`self.K2_GetActorLocation` (`GameplayStatics.GetPlayerPawn` _index)))
          (bind _distance (`self.GetPlaneDistance` _returnvalue_2))
          (if (< _distance 200.0)
            (if (not (> (`KismetMathLibrary.Dot_VectorVector` (`self.NormalVector`) (- _returnvalue_2 (`self.K2_GetActorLocation`))) 0.0))
              (`PrimitiveComponent.SetCollisionEnabled` (`self.Cube`) "NoCollision"))))))))

(event `SetDeleteScale`
  (params (scale :type "Float (double-precision)"))
  (`SceneComponent.SetWorldScale3D` (`self.Cube`) (`KismetMathLibrary.VLerp` (0.0 0.0 0.0) (`self.DefaltScale`) scale)))

(fn `GetPlaneDistance`
  (params (Position :type "Vector Structure"))
  (returns (Distance :type "Float (double-precision)"))
  (return (`KismetMathLibrary.Vector_Distance` Position (`KismetMathLibrary.ProjectPointOnToPlane` Position (`self.K2_GetActorLocation`) (`self.NormalVector`)))))

(fn `UserConstructionScript`)