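; BP_Wall is a wall actor whose material pulses through an animated Alpha parameter while MoveFlag is on.
; BeginPlay creates a dynamic instance of M_Wall on the Cube component and stores it.
; Tick accumulates elapsed time while the flag is set and drives Alpha with an offset, scaled sine wave.
; Nothing in this Blueprint sets MoveFlag or moves the actor.
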(event `self.ReceiveBeginPlay`
  (bind _returnvalue (`PrimitiveComponent.CreateDynamicMaterialInstance` (`self.Cube`) 0 "/Game/BP/Wall/M_Wall.M_Wall" "None"))
  (set `self.Material` _returnvalue))

(event `self.ReceiveTick`
  (params (DeltaSeconds :type "Float (single-precision)"))
  (if (`self.MoveFlag`)
    (bind _output_get (set `self.Time` (+ DeltaSeconds (`self.Time`))))
    (`MaterialInstanceDynamic.SetScalarParameterValue` (`self.Material`) "Alpha" (+ (* (`KismetMathLibrary.Sin` _output_get) 0.7) 1.0))))

(fn `UserConstructionScript`)