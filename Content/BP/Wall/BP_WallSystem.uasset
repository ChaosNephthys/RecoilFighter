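; BP_WallSystem builds walls between pairs of pile actors when play begins.
; For each Pile entry, it spawns a BP_Wall at the midpoint of Pile1 and Pile2, using the look-at yaw and roll but not pitch.
; X scale comes from the piles' 2D distance divided by 100, stretching each wall across the horizontal gap.
; Spawned walls are stored in the Wall array.
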(event `self.ReceiveBeginPlay`
  (for _array_element (`self.Pile`)
    (bind (_pile1 _pile2) (break `/Game/BP/Wall/STR_PilePair` _array_element))
    (bind _returnvalue_location (`KismetMathLibrary.BreakTransform` (`self.GetTransform` _pile1)))
    (bind _returnvalue_location_2 (`KismetMathLibrary.BreakTransform` (`self.GetTransform` _pile2)))
    (bind (_returnvalue_roll _returnvalue_pitch _returnvalue_yaw) (`KismetMathLibrary.BreakRotator` (`KismetMathLibrary.FindLookAtRotation` _returnvalue_location _returnvalue_location_2)))
    (bind _returnvalue (`|SpawnActorFromClass` "/Game/BP/Wall/BP_Wall.BP_Wall_C" (`KismetMathLibrary.MakeTransform` (/ (+ _returnvalue_location _returnvalue_location_2) 2.0) (`KismetMathLibrary.MakeRotator` _returnvalue_roll 0.0 _returnvalue_yaw) (`KismetMathLibrary.MakeVector` (/ (`KismetMathLibrary.Distance2D` (`KismetMathLibrary.Conv_VectorToVector2D` _returnvalue_location) (`KismetMathLibrary.Conv_VectorToVector2D` _returnvalue_location_2)) 100.0) 1.0 1.0)) "Undefined" "OverrideRootScale" null null))
    (`KismetArrayLibrary.Array_Add` (`self.Wall`) _returnvalue)))

(fn `UserConstructionScript`)