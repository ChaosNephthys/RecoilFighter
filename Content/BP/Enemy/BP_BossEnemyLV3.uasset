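; Level 3 boss enemy Blueprint that builds on a parent class, adding range-attack rotation, landing dust and its own shot origin.
; While RangeAttackFlag is set, Tick turns the actor in yaw by a fixed step per frame, independent of delta time.
; LandingCollision overlaps spawn a Niagara dust effect without auto-destroy.
; The construction script sets the RangeAttackPower vector, and GetShotPosition returns the mesh's muzzle socket location.
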(event `self.ReceiveBeginPlay`
  (`parent.ReceiveBeginPlay`))

(event `self.ReceiveTick`
  (params (DeltaSeconds :type "Float (single-precision)"))
  (bind (_returnvalue_roll _returnvalue_pitch _returnvalue_yaw) (`KismetMathLibrary.BreakRotator` (`self.K2_GetActorRotation`)))
  (`parent.ReceiveTick` DeltaSeconds)
  (if (`self.RangeAttackFlag`)
    (`self.K2_SetActorRotation` (`KismetMathLibrary.MakeRotator` _returnvalue_roll _returnvalue_pitch (+ _returnvalue_yaw 1.0)))))

(event `self.LandingCollision.OnComponentBeginOverlap`
  (params (OverlappedComponent :type "PrimitiveComponent Object Reference") (OtherActor :type "Actor Object Reference") (OtherComp :type "PrimitiveComponent Object Reference") (OtherBodyIndex :type Integer) (bFromSweep :type Boolean) (SweepResult :type "HitResult Structure (by ref)"))
  (`NiagaraFunctionLibrary.SpawnSystemAtLocation` "/Game/Effects/N_DustSmork.N_DustSmork" (`SceneComponent.K2_GetComponentLocation` (`self.LandingCollision`)) (struct) (1.0 1.0 1.0) false))

(fn `GetShotPosition`
  (returns (StartPosition :type "Vector Structure"))
  (return (`SceneComponent.GetSocketLocation` (`self.Mesh`) "Muzzle_01")))

(fn `UserConstructionScript`
  (`parent.UserConstructionScript`)
  (set `self.RangeAttackPower` (3000.0 3000.0 5000.0)))