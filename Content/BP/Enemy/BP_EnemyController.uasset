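; Enemy AI controller that tracks which player character is closest to the controlled pawn.
; On BeginPlay it sets up the BB_EnemyAI blackboard and caches all ThirdPersonCharacter actors once.
; Every Tick it scans that cached list by squared 2D distance and writes the closest actor to the NearestPlayer blackboard key.
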(event `self.ReceiveBeginPlay`
  (`self.UseBlackboard` "/Game/BP/Enemy/BB_EnemyAI.BB_EnemyAI")
  (`self.PlayersUpdate`))

(event `self.ReceiveTick`
  (params (DeltaSeconds :type "Float (single-precision)"))
  (bind _nearestplayer (`self.ChackNearestPlayer`))
  (`BlackboardComponent.SetValueAsObject` (`AIBlueprintHelperLibrary.GetBlackboard` null) "NearestPlayer" _nearestplayer))

(fn `ChackNearestPlayer`
  (returns (NearestPlayer :type "/Game/ThirdPersonBP/Blueprints/ThirdPersonCharacter Object Reference"))
  (locals (ret :type "/Game/ThirdPersonBP/Blueprints/ThirdPersonCharacter Object Reference") (distance :type "Float (double-precision)" :default -1.0))
  (bind _distance (`local.distance`))
  (set `local.distance` -1.0)
  (for _array_element (`self.Players`)
    (bind _returnvalue (`KismetMathLibrary.Vector_Distance2DSquared` (`self.K2_GetActorLocation` _array_element) (`self.K2_GetActorLocation` (`self.K2_GetPawn`))))
    (if (or (< _returnvalue _distance) (== _distance -1.0))
      (set `local.ret` _array_element)
      (set `local.distance` _returnvalue)))
  (return (`local.ret`)))

(fn `PlayersUpdate`
  (bind _outactors (`GameplayStatics.GetAllActorsOfClass` "/Game/ThirdPersonBP/Blueprints/ThirdPersonCharacter.ThirdPersonCharacter_C"))
  (set `self.Players` _outactors))

(fn `UserConstructionScript`)