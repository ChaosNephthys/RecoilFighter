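; BP_EnemyBlastBullet is an enemy projectile that flies forward and explodes on contact, damaging and knocking back player characters.
; Tick moves it by ShotSpeed with a swept offset, while a Niagara beam is tinted red and a short lifespan limits range.
; Sphere triggers the blast on overlaps other than BP_AttackWarning.
; Sphere1 defines the blast area for damage, outward impulse and explosion effect scale, then the bullet destroys itself.
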(event `self.ReceiveBeginPlay`
  (`NiagaraComponent.SetVariableLinearColor` (`self.Niagara`) "BeamColor" (`KismetMathLibrary.MakeColor` 100.0))
  (`self.SetLifeSpan` 2.0))

(event `self.Sphere.OnComponentBeginOverlap`
  (params (OverlappedComponent :type "PrimitiveComponent Object Reference") (OtherActor :type "Actor Object Reference") (OtherComp :type "PrimitiveComponent Object Reference") (OtherBodyIndex :type Integer) (bFromSweep :type Boolean) (SweepResult :type "HitResult Structure (by ref)"))
  (bind (_returnvalue_location _returnvalue_rotation _returnvalue_scale) (`KismetMathLibrary.BreakTransform` (`SceneComponent.GetRelativeTransform` (`self.Sphere1`))))
  (cast `/Game/BP/BP_AttackWarning` OtherActor
    (:`CastFailed`
      (for _array_element (`PrimitiveComponent.GetOverlappingActors` (`self.Sphere1`) "/Game/ThirdPersonBP/Blueprints/ThirdPersonCharacter.ThirdPersonCharacter_C")
        (`GameplayStatics.ApplyDamage` _array_element 10.0)
        (bind _asthird_person_character (cast `/Game/ThirdPersonBP/Blueprints/ThirdPersonCharacter` _array_element))
        (`CharacterMovementComponent.AddImpulse` (`Character.CharacterMovement` _asthird_person_character) (* (`KismetMathLibrary.Normal` (- (`self.K2_GetActorLocation` _array_element) (`self.K2_GetActorLocation`))) 1000.0) true))
      (`/Engine/EditorBlueprintResources/StandardMacros.IsValid` (`self.DefaultSceneRoot`)
        (:`Is Valid`
          (`GameplayStatics.SpawnEmitterAtLocation` "/Game/StarterContent/Particles/P_Explosion.P_Explosion" (`self.K2_GetActorLocation`) (struct) (* _returnvalue_scale 0.7))
          (`self.K2_DestroyActor`))))))

(event `self.ReceiveTick`
  (params (DeltaSeconds :type "Float (single-precision)"))
  (bind _defaultsceneroot (`self.DefaultSceneRoot`))
  (`SceneComponent.K2_AddWorldOffset` _defaultsceneroot (* (`SceneComponent.GetForwardVector` _defaultsceneroot) (* DeltaSeconds (`self.ShotSpeed`))) true false))

(fn `UserConstructionScript`)