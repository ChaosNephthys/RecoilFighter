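; BP_FlyEnemy is a flying enemy character that hovers with a gentle vertical bob.
; On BeginPlay it zeroes the movement component's gravity and stores the mesh's relative Z as the baseline.
; Each Tick accumulates time and teleports the mesh's relative Z along a sine wave around that baseline, moving only the mesh rather than the actor.
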(event `self.ReceiveBeginPlay`
  (`parent.ReceiveBeginPlay`)
  (set `CharacterMovementComponent.GravityScale` 0.0 (`self.CharacterMovement`))
  (set `self.DefaltZ` (.z (.location (`SceneComponent.GetRelativeTransform` (`self.Mesh`))))))

(event `self.ReceiveTick`
  (params (DeltaSeconds :type "Float (single-precision)"))
  (`parent.ReceiveTick` DeltaSeconds)
  (set `self.Time` (+ DeltaSeconds (`self.Time`)))
  (`SceneComponent.K2_SetRelativeLocation` (`self.Mesh`) (`KismetMathLibrary.MakeVector` 0.0 0.0 (+ (`self.DefaltZ`) (* 10 (`KismetMathLibrary.Sin` (`self.Time`))))) false true))

(fn `UserConstructionScript`
  (`parent.UserConstructionScript`))