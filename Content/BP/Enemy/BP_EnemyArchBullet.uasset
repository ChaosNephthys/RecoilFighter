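; BP_EnemyArchBullet is a short-lived homing projectile fired by an enemy.
; Each tick it sweeps its root along ShotVector, then updates that vector with a Seek steering function aimed at the target's capsule.
; Overlapping the ThirdPersonCharacter deals damage, and any overlap except with BP_AttackWarning spawns a spark Niagara effect and destroys the bullet.
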(event `self.ReceiveBeginPlay`
  (`NiagaraComponent.SetNiagaraVariableFloat` (`self.Niagara`) "lifeTime" 0.5)
  (`self.SetLifeSpan` 2.5))

(event `self.ReceiveActorBeginOverlap`
  (params (OtherActor :type "Actor Object Reference"))
  (bind _asthird_person_character (cast `/Game/ThirdPersonBP/Blueprints/ThirdPersonCharacter` OtherActor)
    (:`then`
      (`GameplayStatics.ApplyDamage` _asthird_person_character 10.0))
    (:`CastFailed`
      (cast `/Game/BP/BP_AttackWarning` OtherActor
        (:`CastFailed`
          _))))
  (bind _returnvalue (`NiagaraFunctionLibrary.SpawnSystemAtLocation` "/Game/Effects/N_Spark.N_Spark" (`SceneComponent.K2_GetComponentLocation` (`self.DefaultSceneRoot`)) (struct) (1.0 1.0 1.0) false))
  (`NiagaraComponent.SetNiagaraVariableFloat` _returnvalue "maxDistance" 400.0)
  (`self.K2_DestroyActor`))

(event `self.ReceiveTick`
  (params (DeltaSeconds :type "Float (single-precision)"))
  (bind _shotvector (`self.ShotVector`))
  (bind _defaultsceneroot (`self.DefaultSceneRoot`))
  (`SceneComponent.K2_AddWorldOffset` _defaultsceneroot _shotvector true false)
  (`/Engine/EditorBlueprintResources/StandardMacros.IsValid` _defaultsceneroot
    (:`Is Valid`
      (bind _vector (`/Game/BP/Enemy/Steering.Seek` (`SceneComponent.K2_GetComponentLocation` (`Character.CapsuleComponent` (`self.Target`))) (`SceneComponent.K2_GetComponentLocation` _defaultsceneroot) _shotvector 25.0 25.0))
      (set `self.ShotVector` _vector))))

(fn `UserConstructionScript`)