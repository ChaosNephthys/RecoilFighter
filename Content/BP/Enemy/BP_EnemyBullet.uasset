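; BP_EnemyBullet is an enemy projectile that damages the player character on contact.
; Each tick it sweeps its root along ShotVector, without scaling by delta time, while a Niagara effect has its lifetime set at BeginPlay.
; Any sphere overlap applies damage if the actor is a ThirdPersonCharacter, spawns a non-auto-destroyed N_Spark effect with a set max distance, then destroys the bullet.
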(event `self.ReceiveBeginPlay`
  (`NiagaraComponent.SetNiagaraVariableFloat` (`self.Niagara`) "lifeTime" 1.0))

(event `self.Sphere.OnComponentBeginOverlap`
  (params (OverlappedComponent :type "PrimitiveComponent Object Reference") (OtherActor :type "Actor Object Reference") (OtherComp :type "PrimitiveComponent Object Reference") (OtherBodyIndex :type Integer) (bFromSweep :type Boolean) (SweepResult :type "HitResult Structure (by ref)"))
  (bind _asthird_person_character (cast `/Game/ThirdPersonBP/Blueprints/ThirdPersonCharacter` OtherActor)
    (:`then`
      (`GameplayStatics.ApplyDamage` _asthird_person_character 10.0))
    (:`CastFailed`
      _))
  (bind _returnvalue (`NiagaraFunctionLibrary.SpawnSystemAtLocation` "/Game/Effects/N_Spark.N_Spark" (`SceneComponent.K2_GetComponentLocation` (`self.DefaultSceneRoot`)) (struct) (1.0 1.0 1.0) false))
  (`NiagaraComponent.SetNiagaraVariableFloat` _returnvalue "maxDistance" 400.0)
  (`self.K2_DestroyActor`))

(event `self.ReceiveTick`
  (params (DeltaSeconds :type "Float (single-precision)"))
  (`SceneComponent.K2_AddWorldOffset` (`self.DefaultSceneRoot`) (`self.ShotVector`) true false))

(fn `UserConstructionScript`)