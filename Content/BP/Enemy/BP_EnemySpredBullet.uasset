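; BP_EnemySpredBullet is a short-lived enemy projectile that scatters attack warnings around its path as it flies.
; Tick sweeps it forward at ShotSpeed and runs a countdown that spawns a one-second BP_AttackWarning at a random horizontal offset each Span.
; Sphere overlap with ThirdPersonCharacter applies damage, spawns a Niagara spark and destroys the bullet.
; Other overlaps destroy it without a spark, except BP_AttackWarning, which it ignores.
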(event `self.ReceiveBeginPlay`
  (`NiagaraComponent.SetVariableLinearColor` (`self.Niagara`) "BeamColor" (`KismetMathLibrary.MakeColor` 100.0))
  (`self.SetLifeSpan` 2.0))

(event `self.Sphere.OnComponentBeginOverlap`
  (params (OverlappedComponent :type "PrimitiveComponent Object Reference") (OtherActor :type "Actor Object Reference") (OtherComp :type "PrimitiveComponent Object Reference") (OtherBodyIndex :type Integer) (bFromSweep :type Boolean) (SweepResult :type "HitResult Structure (by ref)"))
  (bind _defaultsceneroot (`self.DefaultSceneRoot`))
  (bind _asthird_person_character (cast `/Game/ThirdPersonBP/Blueprints/ThirdPersonCharacter` OtherActor)
    (:`then`
      (`GameplayStatics.ApplyDamage` _asthird_person_character (`self.Damege`))
      (`/Engine/EditorBlueprintResources/StandardMacros.IsValid` _defaultsceneroot
        (:`Is Valid`
          (bind _returnvalue (`NiagaraFunctionLibrary.SpawnSystemAtLocation` "/Game/Effects/N_Spark.N_Spark" (`SceneComponent.K2_GetComponentLocation` _defaultsceneroot) (struct) (1.0 1.0 1.0) false))
          (`NiagaraComponent.SetNiagaraVariableFloat` _returnvalue "maxDistance" 400.0))))
    (:`CastFailed`
      (cast `/Game/BP/BP_AttackWarning` OtherActor
        (:`CastFailed`
          _))))
  (`self.K2_DestroyActor`))

(event `self.ReceiveTick`
  (params (DeltaSeconds :type "Float (single-precision)"))
  (bind _returnvalue (`KismetMathLibrary.GetPI`))
  (bind _defaultsceneroot (`self.DefaultSceneRoot`))
  (bind _returnvalue_2 (- (`self.Time`) DeltaSeconds))
  (`SceneComponent.K2_AddWorldOffset` _defaultsceneroot (* (`SceneComponent.GetForwardVector` _defaultsceneroot) (* DeltaSeconds (`self.ShotSpeed`))) true false)
  (set `self.Time` _returnvalue_2)
  (if (< _returnvalue_2 0.0)
    (set `self.Time` (`self.Span`))
    (bind _returnvalue_3 (`|SpawnActorFromClass` "/Game/BP/BP_AttackWarning.BP_AttackWarning_C" (`KismetMathLibrary.MakeTransform` (+ (`SceneComponent.K2_GetComponentLocation` (`self.DefaultSceneRoot`)) (* (`KismetMathLibrary.MakeVector` (`KismetMathLibrary.Sin` (* (`KismetMathLibrary.RandomFloat`) _returnvalue 2.0)) (`KismetMathLibrary.Cos` (* (`KismetMathLibrary.RandomFloat`) _returnvalue 2.0))) 500.0))) "Undefined" "OverrideRootScale" null null))
    (bind _output_get (set `/Game/BP/BP_AttackWarning.Time` 1.0 _returnvalue_3))
    (set `/Game/BP/BP_AttackWarning.TimeLeft` _output_get _returnvalue_3)))

(fn `UserConstructionScript`)