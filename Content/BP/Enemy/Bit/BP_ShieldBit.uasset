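; BP_ShieldBit is an enemy shield bit, a child Blueprint that relies on inherited behavior.
; BeginPlay sets its Hp and creates a dynamic material on the Cube to tint the emissive parameter light blue.
; Each Tick calls Loop and LookRevOwner, whose names suggest looping movement and facing relative to the owner.
; The overlap event is disabled, and the construction script only calls the parent.
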(event `self.ReceiveBeginPlay`
  (`parent.ReceiveBeginPlay`)
  (set `self.Hp` 300.0)
  (bind _returnvalue (`PrimitiveComponent.CreateDynamicMaterialInstance` (`self.Cube`) 0 null "None"))
  (`MaterialInstanceDynamic.SetVectorParameterValue` _returnvalue "Emmissive" (make `LinearColor` 0.0 0.5 1.0)))

(event `self.ReceiveTick`
  (params (DeltaSeconds :type "Float (single-precision)"))
  (`parent.ReceiveTick` DeltaSeconds)
  (`self.Loop` DeltaSeconds)
  (`self.LookRevOwner`))

(fn `UserConstructionScript`
  (`parent.UserConstructionScript`))