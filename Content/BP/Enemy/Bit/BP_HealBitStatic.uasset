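; BP_HealBitStatic is an enemy heal bit that continuously heals its owner enemy while showing a Niagara beam linked to it.
; BeginPlay resets the beam's end point to zero.
; While the beam component is valid, Tick moves the end to the owner's capsule location and applies healing scaled by delta time for a frame-rate-independent rate.
; OwnerEnemy itself is used without a validity check.
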(event `self.ReceiveBeginPlay`
  (`parent.ReceiveBeginPlay`)
  (`NiagaraComponent.SetNiagaraVariableVec3` (`self.HealConnectBeam`) "Beam End" (0.0 0.0 0.0)))

(event `self.ReceiveTick`
  (params (DeltaSeconds :type "Float (single-precision)"))
  (bind _ownerenemy (`self.OwnerEnemy`))
  (bind _healconnectbeam (`self.HealConnectBeam`))
  (`parent.ReceiveTick` DeltaSeconds)
  (`/Engine/EditorBlueprintResources/StandardMacros.IsValid` _healconnectbeam
    (:`Is Valid`
      (`NiagaraComponent.SetNiagaraVariableVec3` _healconnectbeam "Beam End" (`SceneComponent.K2_GetComponentLocation` (`Character.CapsuleComponent` _ownerenemy)))
      (`/Game/BP/Enemy/BaseEnemy.Heal` _ownerenemy (* DeltaSeconds 20.0)))))

(fn `UserConstructionScript`
  (`parent.UserConstructionScript`))