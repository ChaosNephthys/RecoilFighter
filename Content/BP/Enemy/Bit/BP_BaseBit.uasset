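; BP_BaseBit is a base enemy bit: a destructible satellite that orbits its OwnerEnemy and explodes when it or that owner dies.
; Loop advances a sine/cosine circle around the owner and eases the bit toward it with a swept lerp.
; LookRevOwner faces it away from the owner; neither event is called within this Blueprint.
; Tick watches owner validity and HP, while AnyDamage drains the bit's own HP, both triggering DeathEffect.
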(event `self.ReceiveTick`
  (params (DeltaSeconds :type "Float (single-precision)"))
  (bind _ownerenemy (`self.OwnerEnemy`))
  (`/Engine/EditorBlueprintResources/StandardMacros.IsValid` _ownerenemy
    (:`Is Valid`
      (if (< (`/Game/BP/Enemy/BaseEnemy.HP` _ownerenemy) 0.0)
        (`self.DeathEffect`)))
    (:`Is Not Valid`
      (`self.DeathEffect`))))

(event `Loop`
  (params (Delta :type "Float (double-precision)"))
  (bind _defaultsceneroot (`self.DefaultSceneRoot`))
  (bind _looptime (`self.LoopTime`))
  (`/Engine/EditorBlueprintResources/StandardMacros.IsValid` (`self.OwnerEnemy`)
    (:`Is Valid`
      (set `self.LoopTime` (+ Delta (`self.LoopTime`)))
      (bind _output_get (set `self.TargetPos` (+ (* (`KismetMathLibrary.MakeVector` (`KismetMathLibrary.Sin` _looptime) (`KismetMathLibrary.Cos` _looptime)) (`self.LoopRadius`)) (`self.K2_GetActorLocation` (`self.OwnerEnemy`)))))
      (`/Engine/EditorBlueprintResources/StandardMacros.IsValid` _defaultsceneroot
        (:`Is Valid`
          (`SceneComponent.K2_SetWorldLocation` _defaultsceneroot (`KismetMathLibrary.VLerp` _output_get (`self.K2_GetActorLocation`) 0.95) true false))))))

(event `LookRevOwner`
  (`SceneComponent.K2_SetWorldRotation` (`self.DefaultSceneRoot`) (`KismetMathLibrary.FindLookAtRotation` (`self.K2_GetActorLocation` (`self.OwnerEnemy`)) (`self.K2_GetActorLocation`)) false false))

(event `self.ReceiveAnyDamage`
  (params (Damage :type "Float (single-precision)") (DamageType :type "DamageType Object Reference") (InstigatedBy :type "Controller Object Reference") (DamageCauser :type "Actor Object Reference"))
  (bind _output_get (set `self.Hp` (- (`self.Hp`) Damage)))
  (if (< _output_get 0.0)
    (`self.DeathEffect`)))

(event `DeathEffect`
  (`GameplayStatics.SpawnEmitterAtLocation` "/Game/StarterContent/Particles/P_Explosion.P_Explosion" (`self.K2_GetActorLocation`))
  (`self.K2_DestroyActor`))

(fn `UserConstructionScript`)