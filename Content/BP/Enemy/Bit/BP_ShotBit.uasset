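; BP_ShotBit is an enemy bit that periodically fires predictive shots at the player.
; When the Tick timer passes ShotSpan, a DoOnce draws a red Niagara beam to the predicted player position, calculated from capped velocity, bullet travel time and shot delay.
; After ShotDelayTime it spawns BP_EnemyBullet along the locked aim and resets the timer.
; Outside the firing phase, Tick calls Loop and re-arms the DoOnce.
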(event `self.ReceiveTick`
  (params (DeltaSeconds :type "Float (single-precision)"))
  (bind _returnvalue (`GameplayStatics.GetPlayerPawn` 0))
  (bind _returnvalue_2 (`self.K2_GetActorLocation` _returnvalue))
  (bind _returnvalue_3 (`SceneComponent.K2_GetComponentLocation` (`self.DefaultSceneRoot`)))
  (bind _returnvalue_4 (`self.GetVelocity` _returnvalue))
  (bind _returnvalue_5 (+ _returnvalue_2 (* (* (`KismetMathLibrary.Normal` _returnvalue_4) (`KismetMathLibrary.FMin` (`self.MaxTrackSpeed`) (`KismetMathLibrary.VSize` _returnvalue_4))) (+ (/ (`KismetMathLibrary.Vector_Distance` _returnvalue_2 _returnvalue_3) (`self.BulletSpeed`)) (`self.ShotDelayTime`)))))
  (`parent.ReceiveTick` DeltaSeconds)
  (bind _output_get (set `self.AttackTime` (+ (`self.AttackTime`) DeltaSeconds)))
  (if (> _output_get (`self.ShotSpan`))
    (`/Engine/EditorBlueprintResources/StandardMacros.DoOnce` false :!label _label
      (:`Completed`
        ;[1 1 1] 弾の発射
        (bind _returnvalue_6 (`NiagaraFunctionLibrary.SpawnSystemAtLocation` "/Game/BP/Enemy/BeamPointer.BeamPointer"))
        (`NiagaraComponent.SetNiagaraVariableVec3` _returnvalue_6 "StartPosition" _returnvalue_3)
        (`NiagaraComponent.SetVariableLinearColor` _returnvalue_6 "BeamColor" (`KismetMathLibrary.MakeColor` 100.0))
        (`NiagaraComponent.SetNiagaraVariableVec3` _returnvalue_6 "EndPosition" _returnvalue_5)
        (bind _output_get_2 (set `self.ShotRotate` (`KismetMathLibrary.FindLookAtRotation` (`KismetMathLibrary.Vector_Zero`) (`KismetMathLibrary.Normal` (- _returnvalue_5 _returnvalue_3)))))
        (`KismetSystemLibrary.Delay` (`self.ShotDelayTime`))
        (bind _returnvalue_7 (`|SpawnActorFromClass` "/Game/BP/Enemy/BP_EnemyBullet.BP_EnemyBullet_C" (`KismetMathLibrary.MakeTransform` _returnvalue_3 _output_get_2) "Undefined" "OverrideRootScale" null null))
        (`/Engine/EditorBlueprintResources/StandardMacros.IsValid` _returnvalue_7
          (:`Is Valid`
            (set `/Game/BP/Enemy/BP_EnemyBullet.ShotSpeed` (`self.BulletSpeed`) _returnvalue_7))
          (:`Is Not Valid`
            _))
        (set `self.AttackTime` 0.0)))
    (else
      (`self.Loop` DeltaSeconds)
      (goto _label :!via `Reset`))))

(fn `UserConstructionScript`
  (`parent.UserConstructionScript`))